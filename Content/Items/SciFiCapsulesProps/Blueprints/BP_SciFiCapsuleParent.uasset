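; Parent Blueprint for sci-fi capsule props, letting each capsule set its cap, colors, glow and glass look.
; The Construction Script adds an optional cap mesh at the CapScene location with its own scale.
; It then writes a custom-color toggle, four colors and glass parameters to body and cap materials by parameter name, with emissive settings applied only to the body.
; The event graph has no runtime logic.
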(fn `UserConstructionScript`
  (bind _capmesh (`self.CapMesh`))
  (bind _mesh (`self.Mesh`))
  ;[1 1 1] Edit Material Instance
  (`|ExecutionSequence`
    (:`then_0`
      (`/Engine/EditorBlueprintResources/StandardMacros.IsValid` _capmesh
        (:`Is Valid`
          (bind _returnvalue (`AddComponent|NODE_AddStaticMeshComponent-0` :`RelativeTransform` (`KismetMathLibrary.MakeTransform` (`SceneComponent.RelativeLocation` (`self.CapScene`)) (struct) (`KismetMathLibrary.Conv_DoubleToVector` (`self.CapScale`)))))
          (`StaticMeshComponent.SetStaticMesh` _returnvalue _capmesh))))
    (:`then_1`
      (`MeshComponent.SetScalarParameterValueOnMaterials` _mesh "isCustomColors" (`KismetMathLibrary.Conv_BoolToDouble` (`self.isCustomColors`)))
      (`MeshComponent.SetScalarParameterValueOnMaterials` _returnvalue "isCustomColors" (`KismetMathLibrary.Conv_BoolToDouble` (`self.isCustomColors`))))
    (:`then_2`
      (`MeshComponent.SetVectorParameterValueOnMaterials` _mesh "Color01" (`KismetMathLibrary.Conv_LinearColorToVector` (`self.Color01`)))
      (`MeshComponent.SetVectorParameterValueOnMaterials` _returnvalue "Color01" (`KismetMathLibrary.Conv_LinearColorToVector` (`self.Color01`)))
      (`MeshComponent.SetVectorParameterValueOnMaterials` _mesh "Color02" (`KismetMathLibrary.Conv_LinearColorToVector` (`self.Color02`)))
      (`MeshComponent.SetVectorParameterValueOnMaterials` _returnvalue "Color02" (`KismetMathLibrary.Conv_LinearColorToVector` (`self.Color02`)))
      (`MeshComponent.SetVectorParameterValueOnMaterials` _mesh "Color03" (`KismetMathLibrary.Conv_LinearColorToVector` (`self.Color03`)))
      (`MeshComponent.SetVectorParameterValueOnMaterials` _returnvalue "Color03" (`KismetMathLibrary.Conv_LinearColorToVector` (`self.Color03`)))
      (`MeshComponent.SetVectorParameterValueOnMaterials` _mesh "Color04" (`KismetMathLibrary.Conv_LinearColorToVector` (`self.Color04`)))
      (`MeshComponent.SetVectorParameterValueOnMaterials` _returnvalue "Color04" (`KismetMathLibrary.Conv_LinearColorToVector` (`self.Color04`)))
      (`MeshComponent.SetVectorParameterValueOnMaterials` _mesh "EmissiveColor" (`KismetMathLibrary.Conv_LinearColorToVector` (`self.EmissiveColor`)))
      (`MeshComponent.SetScalarParameterValueOnMaterials` _mesh "EmissivePower" (`self.EmissivePower`))
      (`MeshComponent.SetVectorParameterValueOnMaterials` _mesh "Color" (`KismetMathLibrary.Conv_LinearColorToVector` (`self.GlassColor`)))
      (`MeshComponent.SetVectorParameterValueOnMaterials` _returnvalue "Color" (`KismetMathLibrary.Conv_LinearColorToVector` (`self.GlassColor`)))
      (`MeshComponent.SetScalarParameterValueOnMaterials` _mesh "Metallic" (`self.GlassMetallic`))
      (`MeshComponent.SetScalarParameterValueOnMaterials` _returnvalue "Metallic" (`self.GlassMetallic`))
      (`MeshComponent.SetScalarParameterValueOnMaterials` _mesh "Refraction" (`self.GlassRefraction`))
      (`MeshComponent.SetScalarParameterValueOnMaterials` _returnvalue "Refraction" (`self.GlassRefraction`))
      (`MeshComponent.SetScalarParameterValueOnMaterials` _mesh "Roughness" (`self.GlassRoughness`))
      (`MeshComponent.SetScalarParameterValueOnMaterials` _returnvalue "Roughness" (`self.GlassRoughness`))
      (`MeshComponent.SetScalarParameterValueOnMaterials` _mesh "Opacity_FresnelExponentIn" (`self.GlassOpacity_FresnelExponentIn`))
      (`MeshComponent.SetScalarParameterValueOnMaterials` _returnvalue "Opacity_FresnelExponentIn" (`self.GlassOpacity_FresnelExponentIn`))
      (`MeshComponent.SetScalarParameterValueOnMaterials` _mesh "Opacity_BaseReflectFractionIn" (`self.GlassOpacity_BaseReflectFractionIn`))
      (`MeshComponent.SetScalarParameterValueOnMaterials` _returnvalue "Opacity_BaseReflectFractionIn" (`self.GlassOpacity_BaseReflectFractionIn`)))))